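; B_DebugPlane_b is a debug plane actor whose static mesh bobs vertically in a smooth sine motion.
; Tick accumulates delta time into a counter and sets the mesh's relative location along Z from a sine of that counter.
; The construction script picks a random phase offset, so separate instances can move out of sync.
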(event EventBeginPlay)

(event Collision|EventActorBeginOverlap
  (params (OtherActor :type Actor%20Object%20Reference)))

(event EventTick
  (params (DeltaSeconds :type Float%20%28single-precision%29))
  (bind _output_get (Variables|Default|Setcounter (+ DeltaSeconds (Variables|Default|Getcounter))))
  (Transformation|SetRelativeLocation (Variables|Default|GetStaticMesh) (* "0,0.000000,100.000000" (Math|Trig|Sin(Radians) (* (/ (+ _output_get (Variables|Default|GetRandom)) 4.0) (Math|Trig|GetPI)))) false false))

(fn ConstructionScript
  (Variables|Default|SetRandom (Math|Random|RandomFloatinRange 0.0 1e+01)))